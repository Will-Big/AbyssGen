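; Starter room for AbyssGen that assembles a square room from instanced static meshes in its construction script, with no runtime logic.
; Floor and ceiling are five-by-five grids spaced by S, and each of the four walls leaves its middle segment open.
; Walls share the ceiling's instanced component and rely on the ceiling pass, which runs first, to clear it.
; Wall placement partly uses hard-coded offsets rather than deriving everything from S.
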(fn `UserConstructionScript`
  (bind _s (`self.S`))
  (bind _ism_wallceiling (`self.ISM_WallCeiling`))
  (bind _ism_floor (`self.ISM_Floor`))
  (bind _s_2 (`self.S`))
  (bind _s_3 (`self.S`))
  (`InstancedStaticMeshComponent.ClearInstances` _ism_floor)
  (for _index (range 5)
    (for _index_2 (range 5)
      (`InstancedStaticMeshComponent.AddInstance` _ism_floor (`KismetMathLibrary.MakeTransform` (`KismetMathLibrary.MakeVector` (* _index _s_2) (* _index_2 _s_2))) false)))
  (`InstancedStaticMeshComponent.ClearInstances` _ism_wallceiling)
  (for _index_3 (range 5)
    (for _index_4 (range 5)
      (`InstancedStaticMeshComponent.AddInstance` _ism_wallceiling (`KismetMathLibrary.MakeTransform` (`KismetMathLibrary.MakeVector` (* _index_3 _s) (* _index_4 _s)) (struct :`Roll` 90.0)) false)))
  (for _index_5 (range 5)
    (if (!= _index_5 2)
      (for _ (range 1)
        (`InstancedStaticMeshComponent.AddInstance` (`self.ISM_WallCeiling`) (`KismetMathLibrary.MakeTransform` (`KismetMathLibrary.MakeVector` (* _index_5 (`self.S`)) 0.0 -450.0)) false))))
  (for _index_6 (range 5)
    (if (!= _index_6 2)
      (`InstancedStaticMeshComponent.AddInstance` (`self.ISM_WallCeiling`) (`KismetMathLibrary.MakeTransform` (`KismetMathLibrary.MakeVector` (* _index_6 _s_3) (* _s_3 5.0) -450.0) (struct :`Yaw` 180.0)) false)))
  (for _index_7 (range 5)
    (if (!= _index_7 2)
      (`InstancedStaticMeshComponent.AddInstance` (`self.ISM_WallCeiling`) (`KismetMathLibrary.MakeTransform` (`KismetMathLibrary.MakeVector` -200.0 (+ (* _index_7 (`self.S`)) 200.0) -450.0) (struct :`Yaw` -90.0)) false)))
  (for _index_8 (range 5)
    (if (!= _index_8 2)
      (`InstancedStaticMeshComponent.AddInstance` (`self.ISM_WallCeiling`) (`KismetMathLibrary.MakeTransform` (`KismetMathLibrary.MakeVector` 1800.0 (+ (* _index_8 (`self.S`)) 200.0) -450.0) (struct :`Yaw` 90.0)) false))))